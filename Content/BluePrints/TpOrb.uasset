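; TpOrb is a grabbable VR orb that teleports the player to where it lands when it hits an object named TP_Zone.
; On a valid hit it moves the VRCharacter just above the hit location, keeping its rotation, then returns itself to the character's Sphere2 position with physics off.
; Grab snaps the orb's sphere to the given hand and disables physics, while Drop re-enables physics.
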(event EventGrab
  (params (Hand :type Scene%20Component%20Object%20Reference))
  (Transformation|AttachComponentToComponent (Variables|Default|GetSphere) Hand "None" "SnapToTarget" "SnapToTarget" "KeepWorld" true)
  (Physics|SetSimulatePhysics (Variables|Default|GetSphere) false))

(event Collision|EventHit
  (params (MyComp :type Primitive%20Component%20Object%20Reference) (Other :type Actor%20Object%20Reference) (OtherComp :type Primitive%20Component%20Object%20Reference) (bSelfMoved :type Boolean) (HitLocation :type Vector :default "0, 0, 0") (HitNormal :type Vector :default "0, 0, 0") (NormalImpulse :type Vector :default "0, 0, 0") (Hit :type Hit%20Result%20Structure%20%28by%20ref%29))
  (bind (_x _y _z) (Math|Vector|BreakVector HitLocation))
  (bind _self self)
  (if (Utilities|Enum|Equal(Enum) (Utilities|GetDisplayName Other) "TP_Zone")
    (bind _asvrcharacter (Utilities|Casting|CastToVRCharacter (Game|Player|GetPlayerPawn 0)))
    (Transformation|Teleport _asvrcharacter (Math|Vector|MakeVector _x _y (+ _z 1.5e+02)) (Transformation|GetActorRotation _asvrcharacter))
    (Transformation|Teleport _self (Transformation|GetWorldLocation (Variables|/Game/BluePrints/VRCharacter.VRCharacter_C|GetSphere2 _asvrcharacter)) "0, 0, 0")
    (Physics|SetSimulatePhysics (Variables|Default|GetSphere _self) false)))

(event EventDrop
  (Physics|SetSimulatePhysics (Variables|Default|GetSphere) true))

(fn ConstructionScript)