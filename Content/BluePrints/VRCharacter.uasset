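; VR player character for a paintball game, with motion-controller grabbing, shooting and wall deployment.
; Right trigger press sends a grab message to the first overlapped actor; release drops it through a Gate if still overlapping, otherwise fires a paintball.
; Right grip fires a randomly spread shotgun burst and left trigger spawns a wall at the left hand, both on Delay-based cooldowns.
; Left thumbstick press enables HMD reorientation on controller recenter.
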(event Custom|Release
  (Utilities|FlowControl|Gate true) ; enters at Close
)

(event Input|KeyboardEvents|MotionControllerLeftTrigger
  (params (Key :type Key%20Structure))
  (:Pressed
    (if (Variables|Default|GetSpawnWall?)
      (Variables|Default|SetSpawnWall? false)
      (CallFunction|DeployWall)
      (Utilities|FlowControl|Delay 1e+01)
      (Variables|Default|SetSpawnWall? true))))

(event Input|KeyboardEvents|MotionControllerLeftThumbstick
  (params (Key :type Key%20Structure))
  (:Pressed
    (Class|OculusFunctionLibrary|SetReorientHMDonControllerRecenter true)))

(event Input|KeyboardEvents|MotionControllerRightTrigger
  (params (Key :type Key%20Structure))
  (:Pressed
    (bind _output_get (Variables|Default|SetOverlapped%20Actor (Utilities|Array|Get(acopy) (Collision|GetOverlappingActors (Variables|Default|GetRight) 0 :!class /Script/Engine.PrimitiveComponent))))
    (Class|Interactables|Grab(Message) _output_get (Variables|Default|GetRightHand))
    (goto _label Open))
  (:Released
    (if (Collision|IsOverlappingActor (Variables|Default|GetOverlapped%20Actor) :!class /Script/Engine.Actor)
      (Utilities|FlowControl|Gate true :!label _label
        (:Exit
          (Transformation|DetachFromActor (Variables|Default|GetOverlapped%20Actor) "KeepWorld" "KeepWorld" "KeepWorld")
          (CallFunction|Release)
          (Class|Interactables|Drop(Message) (Variables|Default|GetOverlapped%20Actor))))
      (else
        (CallFunction|Shoot)))))

(event Input|KeyboardEvents|MotionControllerRightGrip1
  (params (Key :type Key%20Structure))
  (:Pressed
    (if (Variables|Default|GetShotgun?)
      (Variables|Default|SetShotgun? false)
      (CallFunction|ShotgunBlast)
      (Utilities|FlowControl|Delay 5.0)
      (Variables|Default|SetShotgun? true))))

(fn ConstructionScript)

(fn Shoot
  (bind _right (Variables|Default|GetRight))
  (bind _returnvalue (Transformation|GetWorldLocation _right))
  (bind _returnvalue_2 (Transformation|GetWorldRotation _right))
  (bind (_roll _pitch _yaw) (Math|Rotator|BreakRotator _returnvalue_2))
  (bind (_x _y _z) (Math|Vector|BreakVector _returnvalue))
  (Game|SpawnActorfromClass "/Game/BluePrints/Paintball.Paintball_C" (Math|Transform|MakeTransform (Math|Vector|MakeVector (+ _x 1e+01) _y _z) (Math|Rotator|MakeRotator _roll (+ _pitch 7.0) _yaw) "0.200000,0.200000,0.200000") "Undefined" 0 0))

(fn DeployWall
  (bind _lefthand (Variables|Default|GetLeftHand))
  (bind _returnvalue (Transformation|GetWorldLocation _lefthand))
  (bind _returnvalue_2 (Transformation|GetWorldRotation _lefthand))
  (bind (_x _y _z) (Math|Vector|BreakVector _returnvalue))
  (bind (_roll _pitch _yaw) (Math|Rotator|BreakRotator _returnvalue_2))
  (Game|SpawnActorfromClass "/Game/BluePrints/WallDeployable.WallDeployable_C" (Math|Transform|MakeTransform (Math|Vector|MakeVector _x _y (+ _z 1e+01)) (Math|Rotator|MakeRotator (+ _pitch 9e+01) 0.0 (+ _yaw 9e+01)) "15.000000,12.000000,1.000000") "Undefined" 0 0))

(fn ShotgunBlast
  (bind _right (Variables|Default|GetRight))
  (bind _returnvalue (Transformation|GetWorldLocation _right))
  (bind _returnvalue_2 (Transformation|GetWorldRotation _right))
  (bind (_roll _pitch _yaw) (Math|Rotator|BreakRotator _returnvalue_2))
  (bind (_x _y _z) (Math|Vector|BreakVector _returnvalue))
  (for _index (range 1 10)
    (Game|SpawnActorfromClass "/Game/BluePrints/Paintball.Paintball_C" (Math|Transform|MakeTransform (Math|Vector|MakeVector (+ _x 1e+01) _y _z) (Math|Rotator|MakeRotator (Math|Random|RandomFloatinRange (- _roll 3.0) (+ _roll 3.0)) (Math|Random|RandomFloatinRange (- _pitch 3.0) (+ _pitch 3.0)) (Math|Random|RandomFloatinRange (- _yaw 3.0) (+ _yaw 3.0))) "0.100000,0.100000,0.100000") "Undefined" 0 0)))