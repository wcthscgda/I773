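; WallDeployable is a short-lived actor, apparently a deployable wall, that destroys itself a few seconds after it spawns.
; BeginPlay runs a fixed chain of Delay nodes that briefly hides and re-shows the static mesh about once a second, producing blinks over its lifetime.
; After the last blink and a short pause, the chain calls DestroyActor.
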(event EventBeginPlay
  (Utilities|FlowControl|Delay 1.0)
  (Rendering|SetVisibility (Variables|Debug|GetStaticMeshComponent) false false)
  (Utilities|FlowControl|Delay 0.05)
  (Rendering|SetVisibility (Variables|Debug|GetStaticMeshComponent) true false)
  (Utilities|FlowControl|Delay 1.0)
  (Rendering|SetVisibility (Variables|Debug|GetStaticMeshComponent) false false)
  (Utilities|FlowControl|Delay 0.03)
  (Rendering|SetVisibility (Variables|Debug|GetStaticMeshComponent) true false)
  (Utilities|FlowControl|Delay 1.0)
  (Rendering|SetVisibility (Variables|Debug|GetStaticMeshComponent) false false)
  (Utilities|FlowControl|Delay 0.03)
  (Rendering|SetVisibility (Variables|Debug|GetStaticMeshComponent) true false)
  (Utilities|FlowControl|Delay 1.0)
  (Rendering|SetVisibility (Variables|Debug|GetStaticMeshComponent) false false)
  (Utilities|FlowControl|Delay 0.03)
  (Rendering|SetVisibility (Variables|Debug|GetStaticMeshComponent) true false)
  (Utilities|FlowControl|Delay 0.5)
  (Actor|DestroyActor))

(fn ConstructionScript)